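; Hero gameplay ability for the light special attack slot; it currently drives only the UI and contains no attack logic.
; On activation it tells the HeroUIComponent to update the slot icon and begin the cooldown display, then ends immediately.
; Small getter functions supply the input tag, icon material and fixed cooldown duration, with no cooldown commit in this graph.
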(event `self.K2_ActivateAbility`
  (bind _returnvalue (`self.GetSpecialAbilityInputTag`))
  (bind _herouicomponent (`WarriorHeroCharacter.HeroUIComponent` (`self.GetWarriorHeroCharacterFromActorInfo`)))
  (`HeroUIComponent.OnSpecialAbilityIconSlotUpdated` _herouicomponent _returnvalue (`self.GetSpecialAbilityIconMaterial`))
  (`HeroUIComponent.OnAbilityCoolDownBegin` _herouicomponent _returnvalue (`self.GetCoolDownDuration`) (`self.GetCoolDownDuration`))
  (`self.K2_EndAbility`))

(event `self.K2_OnEndAbility`
  (params (bWasCancelled :type Boolean)))

(fn `GetCoolDownDuration`
  (returns (ReturnValue :type "Float (single-precision)"))
  (return 8.0))

(fn `GetSpecialAbilityIconMaterial`
  (returns (ReturnValue :type "MaterialInterface Soft Object Reference"))
  (return (`self.SpecialAbilityIconMaterial`)))

(fn `GetSpecialAbilityInputTag`
  (returns (ReturnValue :type "GameplayTag Structure"))
  (return (`BlueprintGameplayTagLibrary.MakeLiteralGameplayTag` (struct :`TagName` "Input.SpecialAbility.Light"))))