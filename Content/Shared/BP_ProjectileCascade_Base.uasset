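; BP_ProjectileCascade_Base is a projectile Blueprint that handles sound and Cascade particle effects for launch, flight and impact.
; On BeginPlay it plays a spawn sound, attaches a flying sound that stops with the actor, and spawns a muzzle emitter along its forward vector.
; OnSpawnProjectileHitFX plays the hit sound and impact emitter at the supplied location.
; Each asset is validity-checked, and the graph contains no movement or damage logic.
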(event `self.ReceiveBeginPlay`
  (`|ExecutionSequence`
    (:`then_0`
      (bind _projectile_spawn_sound (`self.Projectile Spawn Sound`)
        (:`then`
          (`GameplayStatics.PlaySoundAtLocation` _projectile_spawn_sound (`self.K2_GetActorLocation`) (struct) 1.0 1.0 0.0 null null null null))
        (:`else`)))
    (:`then_1`
      (bind _projectike_flying_sound (`self.Projectike Flying Sound`)
        (:`then`
          (`GameplayStatics.SpawnSoundAttached` _projectike_flying_sound (`self.RootComponent`) "None" (0.0 0.0 0.0) (struct) "KeepRelativeOffset" true 1.0 1.0 0.0 null null))
        (:`else`)))
    (:`then_2`
      (bind _projectile_muzzle__effect (`self.Projectile Muzzle  Effect`)
        (:`then`
          (`GameplayStatics.SpawnEmitterAtLocation` _projectile_muzzle__effect (`self.K2_GetActorLocation`) (`KismetMathLibrary.Conv_VectorToRotator` (`self.GetActorForwardVector`))))
        (:`else`)))))

(event `self.BP_OnSpawnProjectileHitFX`
  (params (HitLocation :type "Vector Structure (by ref)"))
  (`|ExecutionSequence`
    (:`then_0`
      (bind _sound_to_play_on_hit (`self.Sound To Play On Hit`)
        (:`then`
          (`GameplayStatics.PlaySoundAtLocation` _sound_to_play_on_hit HitLocation (struct) 1.0 1.0 0.0 null null null null))
        (:`else`)))
    (:`then_1`
      (bind _impacthitfx (`self.ImpactHitFX`)
        (:`then`
          (`GameplayStatics.SpawnEmitterAtLocation` _impacthitfx HitLocation))
        (:`else`)))))

(fn `UserConstructionScript`)